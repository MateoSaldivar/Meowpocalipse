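; Prototype player character: a flipbook sprite that moves relative to the camera, aims a laser at the cursor and sends cats at zombies.
; Q and E step the spring arm in 90-degree turns on Tick, which also picks directional walk or idle animations and records camera facing.
; A trace from actor to cursor hit sets the laser end and caches any targeted zombie for left-click.
; Damage events briefly flash the sprite red.
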(event Custom|TakeDamage
  (bind _sprite (Variables|Default|GetSprite))
  (Sprite|SetSpriteColor _sprite "(R=1.000000,G=0.000000,B=0.000000,A=1.000000)")
  (Utilities|FlowControl|Delay 0.2)
  (Sprite|SetSpriteColor _sprite "(R=1.000000,G=1.000000,B=1.000000,A=1.000000)"))

(event Custom|GetNextRot
  (params (p_bool :type Boolean))
  (if p_bool
    (Variables|Default|SetlimitRot (Math|Conversions|ToFloat(Integer) (Math|Float|Round (+ (.yaw (Transformation|GetWorldRotation (Variables|Default|GetSpringArm))) 9e+01))))
    (Variables|Default|SetstartRightRot true)
    (Variables|Default|SetstartLeftRot false)
    (else
      (Variables|Default|SetlimitRot (Math|Conversions|ToFloat(Integer) (Math|Float|Round (- (.yaw (Transformation|GetWorldRotation (Variables|Default|GetSpringArm))) 9e+01))))
      (Variables|Default|SetstartLeftRot true)
      (Variables|Default|SetstartRightRot false))))

(event Input|EnhancedActionEvents|EnhancedInputActionProtoXYMovement
  (params (ActionValue :type Vector%202D%20Structure) (ElapsedSeconds :type Float%20%28double-precision%29) (TriggeredSeconds :type Float%20%28double-precision%29) (InputAction :type Input%20Action%20Object%20Reference :default "/Game/Input/ProtoXYMovement.ProtoXYMovement"))
  (bind _camera (Variables|Default|GetCamera))
  ;[1 1 1] Movement
  (:Triggered
    (Pawn|Input|AddMovementInput (Math|Vector|GetRightVector _camera) (.x ActionValue) false)
    (Pawn|Input|AddMovementInput (Math|Vector|GetForwardVector _camera) (.y ActionValue) false)))

(event Input|EnhancedActionEvents|EnhancedInputActionELetter
  (params (ActionValue :type Boolean) (ElapsedSeconds :type Float%20%28double-precision%29) (TriggeredSeconds :type Float%20%28double-precision%29) (InputAction :type Input%20Action%20Object%20Reference :default "/Game/Input/ELetter.ELetter"))
  (:Triggered
    (if (not (Variables|Default|GetstartRightRot))
      (if (not (Variables|Default|GetstartLeftRot))
        (CallFunction|GetNextRot true)))))

(event Input|EnhancedActionEvents|EnhancedInputActionQLetter
  (params (ActionValue :type Boolean) (ElapsedSeconds :type Float%20%28double-precision%29) (TriggeredSeconds :type Float%20%28double-precision%29) (InputAction :type Input%20Action%20Object%20Reference :default "/Game/Input/QLetter.QLetter"))
  (:Triggered
    (if (not (Variables|Default|GetstartRightRot))
      (if (not (Variables|Default|GetstartLeftRot))
        (CallFunction|GetNextRot false)))))

(event Collision|EventActorBeginOverlap
  (params (OtherActor :type Actor%20Object%20Reference)))

(event EventTick
  (params (DeltaSeconds :type Float%20%28single-precision%29))
  (CallFunction|Animate)
  (CallFunction|CameraDirections)
  (CallFunction|UpdateSecondRotation)
  (CallFunction|UpdateLaserBeam))

(event EventBeginPlay
  (bind _asplayer_controller (Utilities|Casting|CastToPlayerController (Pawn|GetController)))
  (Input|AddMappingContext (PlayerController|LocalPlayerSubsystems|GetEnhancedInputLocalPlayerSubsystem _asplayer_controller) "/Game/Input/ControllerMap.ControllerMap" 0 "(bIgnoreAllPressedKeysUntilRelease=True,bForceImmediately=False)")
  (Effects|Components|ParticleSystem|SetColorParameter (Variables|Default|GetLaser) "Color" "(R=1.000000,G=0.084660,B=0.000000,A=1.000000)")
  (CallFunction|SetUpCharacter)
  (EventDispatchers|BindEventtoOnStatsTakeDamage (Variables|Default|GetActorStats) (delegate Custom|TakeDamage)))

(event Input|MouseEvents|LeftMouseButton
  (params (Key :type Key%20Structure))
  (:Pressed
    (if (Utilities|IsValid (Variables|Default|GetzombieRef))
      (Default|SendCattoZombie (Variables|Default|GetCatContainer) (Variables|Default|GetzombieRef)))))

(fn ConstructionScript)

(fn UpdateLaserBeam
  (bind _returnvalue (Game|GetPlayerController 0))
  (bind _laser (Variables|Default|GetLaser))
  (bind _laser_2 (Variables|Default|GetLaser))
  (bind (_hitresult _returnvalue_2) (Game|Player|GetHitResultUnderCursorbyChannel _returnvalue "TraceTypeQuery1" true))
  (bind _location (Collision|BreakHitResult _hitresult))
  (if _returnvalue_2
    (Rendering|SetVisibility _laser true false)
    (bind (_outhit _returnvalue_3) (Collision|LineTraceByChannel (Transformation|GetActorLocation) _location "TraceTypeQuery2" true 0 "None"))
    (if _returnvalue_3
      (Effects|Components|ParticleSystem|SetVectorParameter _laser_2 "LaserEnd" (.Location (Collision|BreakHitResult _outhit)))
      (if (Actor|ActorHasTag (.HitActor (Collision|BreakHitResult _outhit)) "Zombie")
        (bind _aszombie_bp (Utilities|Casting|CastToZombieBP (.HitActor (Collision|BreakHitResult _outhit))))
        (Variables|Default|SetzombieRef _aszombie_bp)
        (else
          (Variables|Default|SetzombieRef 0)))
      (else
        (Effects|Components|ParticleSystem|SetVectorParameter _laser_2 "LaserEnd" _location)))
    (else
      (Rendering|SetVisibility _laser false false))))

(fn UpdateSecondRotation
  (bind _springarm (Variables|Default|GetSpringArm))
  (bind _springarm_2 (Variables|Default|GetSpringArm))
  (bind _returnvalue (Transformation|GetWorldRotation _springarm))
  (bind _returnvalue_2 (Transformation|GetWorldRotation _springarm_2))
  (if (Variables|Default|GetstartRightRot)
    (if (== (Variables|Default|GetlimitRot) 2.7e+02)
      (Variables|Default|SetlimitRot -9e+01))
    (bind _output_get (Variables|Default|SetcurrentAngle (+ (.yaw _returnvalue_2) (Variables|Default|GetrotationSpeed))))
    (Transformation|SetWorldRotation (Variables|Default|GetSpringArm) (Math|Rotator|MakeRotator (.roll _returnvalue_2) (.pitch _returnvalue_2) _output_get) false false)
    (if (== (Variables|Default|GetcurrentAngle) (Variables|Default|GetlimitRot))
      (Variables|Default|SetstartRightRot false)
      (Variables|Default|SetstartLeftRot false))
    (elif (Variables|Default|GetstartLeftRot)
      (if (== (Variables|Default|GetlimitRot) -2.7e+02)
        (Variables|Default|SetlimitRot 9e+01))
      (bind _output_get_2 (Variables|Default|SetcurrentAngle (- (.yaw _returnvalue) (Variables|Default|GetrotationSpeed))))
      (Transformation|SetWorldRotation (Variables|Default|GetSpringArm) (Math|Rotator|MakeRotator (.roll _returnvalue) (.pitch _returnvalue) _output_get_2) false false)
      (if (== (Variables|Default|GetcurrentAngle) (Variables|Default|GetlimitRot))
        (Variables|Default|SetstartLeftRot false)
        (Variables|Default|SetstartRightRot false)))))

(fn SetUpCharacter
  (bind _capsulecomponent (Variables|Collision|GetCapsuleComponent))
  (Variables|/Script/Engine.PlayerController|SetbShowMouseCursor (Game|GetPlayerController 0) true)
  (if (> (Variables|Default|GetrotationSpeed) 15.0)
    (Variables|Default|SetrotationSpeed 15.0))
  (Transformation|SetRelativeRotation _capsulecomponent "0, 0, 0" false false)
  (Development|PrintString (Utilities|String|ToString(Float) (.yaw (Transformation|GetWorldRotation _capsulecomponent)))))

(fn Animate
  (bind _returnvalue (Input|EnhancedActionValues|GetProtoXYMovement))
  (bind _animations (LocalVariables|GetAnimations))
  ;[1 1 1] Is the character moving?
  (LocalVariables|SetlocalUpOrDown (.y _returnvalue))
  (LocalVariables|SetlocalRightOrLeft (.x _returnvalue))
  (if (or (!= (LocalVariables|GetlocalUpOrDown) 0.0) (!= (LocalVariables|GetlocalRightOrLeft) 0.0))
    (Variables|Default|SetMoveDirection (select (> (LocalVariables|GetlocalRightOrLeft) 0.5) "NewEnumerator3" (select (< (LocalVariables|GetlocalRightOrLeft) -0.5) "NewEnumerator2" (select (and (< (LocalVariables|GetlocalUpOrDown) -0.5) (== (LocalVariables|GetlocalRightOrLeft) 0.0)) "NewEnumerator1" "NewEnumerator0")))))
  (Sprite|SetFlipbook (Variables|Default|GetSprite) (select (> (Math|Vector|VectorLength (Transformation|GetVelocity)) 0.0) (Utilities|Select :Index (Variables|Default|GetMoveDirection) :NewEnumerator0 (.moveup _animations) :NewEnumerator1 (.movedown _animations) :NewEnumerator2 (.moveleft _animations) :NewEnumerator3 (.moveright _animations)) (Utilities|Select :Index (Variables|Default|GetMoveDirection) :NewEnumerator0 (.idleup _animations) :NewEnumerator1 (.idledown _animations) :NewEnumerator2 (.idleleft _animations) :NewEnumerator3 (.idleright _animations)))))

(fn CameraDirections
  (bind _camera (Variables|Default|GetCamera))
  (bind _returnvalue (Transformation|GetWorldRotation _camera))
  (bind _returnvalue_2 (Math|Float|Round (.yaw _returnvalue)))
  (if (== _returnvalue_2 0)
    (Variables|Default|SetCurrentDirection "NewEnumerator0")
    (elif (== _returnvalue_2 9e+01)
      (Variables|Default|SetCurrentDirection "NewEnumerator1")
      (elif (== (Math|Integer|Absolute(Integer) _returnvalue_2) 1.8e+02)
        (Variables|Default|SetCurrentDirection "NewEnumerator2")
        (elif (== _returnvalue_2 -9e+01)
          (Variables|Default|SetCurrentDirection "NewEnumerator3"))))))

(fn SpendMoney
  (params (Money :type Integer))
  (bind _output_get (Variables|Default|SetMoney (- (Variables|Default|GetMoney) Money)))
  (return _output_get))