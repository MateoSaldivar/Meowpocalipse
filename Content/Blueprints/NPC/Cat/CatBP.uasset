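; Cat NPC character with a 2D flipbook sprite that attacks a zombie target.
; CallAttack stores the target, passes it to CatController and clears IsOwned, which switches a custom trace channel from Block to Overlap.
; While the target overlaps AttackRange, Tick deals ActorStats damage on a cooldown.
; Animation remaps world velocity by the player's CurrentDirection to choose camera-relative directional idle or walk flipbooks.
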(event OnComponentBeginOverlap(attackRange)
  (params (OverlappedComponent :type Primitive%20Component%20Object%20Reference) (OtherActor :type Actor%20Object%20Reference) (OtherComp :type Primitive%20Component%20Object%20Reference) (OtherBodyIndex :type Integer) (bFromSweep :type Boolean) (SweepResult :type Hit%20Result%20Structure%20%28by%20ref%29))
  (if (== OtherActor (Variables|Default|GetZombie))
    (Variables|Default|SetInAttackRange true)))

(event OnComponentEndOverlap(attackRange)
  (params (OverlappedComponent :type Primitive%20Component%20Object%20Reference) (OtherActor :type Actor%20Object%20Reference) (OtherComp :type Primitive%20Component%20Object%20Reference) (OtherBodyIndex :type Integer))
  (if (== OtherActor (Variables|Default|GetZombie))
    (Variables|Default|SetInAttackRange false)))

(event Custom|CallAttack
  (params (Zombie :type Zombie%20BP%20Object%20Reference))
  (bind _ascat_controller (Utilities|Casting|CastToCatController (Pawn|GetController)))
  (Default|Attack _ascat_controller Zombie)
  (Variables|Default|SetZombie Zombie)
  (Variables|Default|SetIsOwned false))

(event EventBeginPlay
  (Default|SetStats (Variables|Default|GetActorStats) (Variables|Character|GetCharacterMovement) (Variables|Default|GetattackRange)))

(event EventTick
  (params (DeltaSeconds :type Float%20%28single-precision%29))
  (CallFunction|Animate)
  (|SetCollider)
  (|Attack DeltaSeconds))

(fn ConstructionScript)

(fn DealDamage
  (Default|StatsTakeDamage (Actor|GetComponentbyClass (Variables|Default|GetZombie) "/Game/Blueprints/NPC/Components/ActorStats.ActorStats_C") (Variables|/Game/Blueprints/NPC/Components/ActorStats.ActorStats_C|GetAttack (Variables|Default|GetActorStats)))
  (if (not (Utilities|IsValid (Variables|Default|GetZombie)))
    (Variables|Default|SetZombie 0)))

(fn Animate
  (bind _animations (LocalVariables|GetAnimations))
  (CallFunction|GetVelwithCamera)
  (if (or (!= (Variables|Default|GetLocalVelX) 0.0) (!= (Variables|Default|GetLocalVelY) 0.0))
    (Variables|Default|SetMoveDirection (select (and (> (Variables|Default|GetLocalVelX) 0.5) (> (Math|Float|Absolute(Float) (Variables|Default|GetXtrueVelocity)) 1e+02)) "NewEnumerator3" (select (and (< (Variables|Default|GetLocalVelX) -0.5) (> (Math|Float|Absolute(Float) (Variables|Default|GetXtrueVelocity)) 1e+02)) "NewEnumerator2" (select (< (Variables|Default|GetLocalVelY) -0.5) "NewEnumerator1" "NewEnumerator0")))))
  (Sprite|SetFlipbook (Variables|Default|GetCat1_F) (select (> (Math|Vector|VectorLength (Transformation|GetVelocity)) 0.0) (Utilities|Select :Index (Variables|Default|GetMoveDirection) :NewEnumerator0 (.moveup _animations) :NewEnumerator1 (.movedown _animations) :NewEnumerator2 (.moveleft _animations) :NewEnumerator3 (.moveright _animations)) (Utilities|Select :Index (Variables|Default|GetMoveDirection) :NewEnumerator0 (.idleup _animations) :NewEnumerator1 (.idledown _animations) :NewEnumerator2 (.idleleft _animations) :NewEnumerator3 (.idleright _animations)))))

(fn GetVelwithCamera
  (bind _asprototype (Utilities|Casting|CastToPrototype (Game|GetPlayerCharacter 0)))
  (if (== (Variables|/Game/Blueprints/Agents/Prototype.Prototype_C|GetCurrentDirection _asprototype) 1)
    (bind _vel (CallFunction|VelocityDecision false 1.0 -1.0))
    (Variables|Default|SetLocalVelX _vel)
    (bind _vel_2 (CallFunction|VelocityDecision true 1.0 -1.0))
    (Variables|Default|SetLocalVelY _vel_2)
    (Variables|Default|SetXtrueVelocity (.y (Transformation|GetVelocity)))
    (elif (== (Variables|/Game/Blueprints/Agents/Prototype.Prototype_C|GetCurrentDirection _asprototype) 2)
      (bind _vel_3 (CallFunction|VelocityDecision true -1.0 1.0))
      (Variables|Default|SetLocalVelX _vel_3)
      (bind _vel_4 (CallFunction|VelocityDecision false 1.0 -1.0))
      (Variables|Default|SetLocalVelY _vel_4)
      (Variables|Default|SetXtrueVelocity (.x (Transformation|GetVelocity)))
      (elif (== (Variables|/Game/Blueprints/Agents/Prototype.Prototype_C|GetCurrentDirection _asprototype) 3)
        (bind _vel_5 (CallFunction|VelocityDecision false -1.0 1.0))
        (Variables|Default|SetLocalVelX _vel_5)
        (bind _vel_6 (CallFunction|VelocityDecision true -1.0 1.0))
        (Variables|Default|SetLocalVelY _vel_6)
        (Variables|Default|SetXtrueVelocity (.y (Transformation|GetVelocity)))
        (elif (== (Variables|/Game/Blueprints/Agents/Prototype.Prototype_C|GetCurrentDirection _asprototype) 4)
          (bind _vel_7 (CallFunction|VelocityDecision true 1.0 -1.0))
          (Variables|Default|SetLocalVelX _vel_7)
          (bind _vel_8 (CallFunction|VelocityDecision false -1.0 1.0))
          (Variables|Default|SetLocalVelY _vel_8)
          (Variables|Default|SetXtrueVelocity (.x (Transformation|GetVelocity))))))))

(fn VelocityDecision
  (params (IsX :type Boolean) (true :type Float%20%28double-precision%29) (false :type Float%20%28double-precision%29))
  (if IsX
    (return (select (== (Math|Float|Round (.x (Transformation|GetVelocity))) 0) 0.0 (select (> (Math|Float|Round (.x (Transformation|GetVelocity))) 0.5) true false)))
    (else
      (return (select (== (Math|Float|Round (.y (Transformation|GetVelocity))) 0) 0.0 (select (> (Math|Float|Round (.y (Transformation|GetVelocity))) 0.5) true false))))))