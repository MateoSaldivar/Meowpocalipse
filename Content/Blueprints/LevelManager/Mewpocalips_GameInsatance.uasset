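; Game instance Blueprint that plays and stops a 2D sound, such as audio meant to carry across level changes.
; PlayAudio creates the sound with a given volume and optional persistence across level transitions, stores the component, starts it and fades it in.
; StopAudio checks that the stored component is valid, fades it out over the given duration and schedules a delayed stop shortly afterward.
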(fn PlayAudio
  (params (Audio :type Sound%20Base%20Object%20Reference) (Volume :type Float%20%28double-precision%29) (Persist :type Boolean))
  (bind _returnvalue (Audio|CreateSound2D Audio Volume 1.0 0.0 0 Persist))
  (bind _output_get (Variables|Default|SetAudio _returnvalue))
  (Audio|Components|Audio|Play _output_get 0.0)
  (Audio|Components|Audio|FadeIn _output_get 2.0 1.0 0.0 "Linear" :!class /Script/Engine.AudioComponent))

(fn StopAudio
  (params (FadeDuration :type Float%20%28double-precision%29))
  (bind _audio (Variables|Default|GetAudio))
  (if (Utilities|IsValid (Variables|Default|GetAudio))
    (Audio|Components|Audio|FadeOut _audio FadeDuration 0.0 "Linear" :!class /Script/Engine.AudioComponent)
    (Audio|Components|Audio|StopDelayed _audio (+ FadeDuration 1.0))))