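; ZombieSpawnerBP is a level spawner that creates a batch of zombie actors at its own transform, staggered over time.
; StartSpawning passes NumEnemies to SpawnZombies, which fires the SpawEnemies event only when CanSpawn is true.
; That event uses a ForLoopWithDelay to spawn ZombiePrefab once per iteration, setting the loop's Delay variable to SpawnRate after each spawn.
; BeginPlay and Tick are empty, so spawning relies on an external call.
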(event Custom|SpawEnemies
  (params (N :type Integer))
  (Utilities|ForLoopwithDelay 0 (- N 1) (Variables|Default|GetDelay)
    (:Loop%20Body
      (Game|SpawnActorfromClass (Variables|Default|GetZombiePrefab) (Transformation|GetActorTransform) "Undefined" "MultiplyWithRoot" 0 0)
      (Variables|Default|SetDelay (Variables|Default|GetSpawnRate)))))

(event EventBeginPlay)

(event Collision|EventActorBeginOverlap
  (params (OtherActor :type Actor%20Object%20Reference)))

(event EventTick
  (params (DeltaSeconds :type Float%20%28single-precision%29)))

(fn ConstructionScript)

(fn SpawnZombies
  (params (NumZombies :type Integer))
  (if (Variables|Default|GetCanSpawn)
    (CallFunction|SpawEnemies NumZombies)))

(fn StartSpawning
  (CallFunction|SpawnZombies (Variables|Default|GetNumEnemies)))