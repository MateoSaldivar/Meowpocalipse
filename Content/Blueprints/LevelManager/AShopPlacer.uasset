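; Level manager actor that places the shop merchant at the spawn point nearest the player.
; On BeginPlay it caches every AShopSpawnPoint in the level.
; SpawnStoreClosestToPlayer picks the closest point in the player's current area by squared distance, then calls ShowMerchant on the Shop with that transform.
; The stored ClosestDistance serves as the search threshold and is not reset between searches here.
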(event EventBeginPlay
  (bind _outactors (Actor|GetAllActorsOfClass "/Game/Blueprints/LevelManager/AShopSpawnPoint.AShopSpawnPoint_C"))
  (Variables|Default|SetSpawnPoints _outactors))

(event Collision|EventActorBeginOverlap
  (params (OtherActor :type Actor%20Object%20Reference)))

(event EventTick
  (params (DeltaSeconds :type Float%20%28single-precision%29)))

(fn ConstructionScript)

(fn GetClosestTransformtoPlayer
  (bind _asprototype (Utilities|Casting|CastToPrototype (Game|GetPlayerCharacter 0)))
  (LocalVariables|SetPlayerPosition (Transformation|GetActorLocation _asprototype))
  (|SetPlayer)
  (for _array_element (Variables|Default|GetSpawnPoints)
    (bind _asashop_spawn_point (Utilities|Casting|CastToAShopSpawnPoint _array_element))
    (if (== (Variables|/Game/Blueprints/LevelManager/AShopSpawnPoint.AShopSpawnPoint_C|GetArea _asashop_spawn_point) (Variables|/Game/Blueprints/Agents/Prototype.Prototype_C|GetCurrentArea (LocalVariables|Getplayer)))
      (if (< (Class|KismetMathLibrary|VectorDistanceSquared (LocalVariables|GetPlayerPosition) (.Location (Math|Transform|BreakTransform (Transformation|GetActorTransform _array_element)))) (LocalVariables|GetClosest%20Distance))
        (LocalVariables|SetClosest%20Distance (Class|KismetMathLibrary|VectorDistanceSquared (LocalVariables|GetPlayerPosition) (.Location (Math|Transform|BreakTransform (Transformation|GetActorTransform _array_element)))))
        (LocalVariables|SetClosestTransform _array_element))))
  (return (LocalVariables|GetClosestTransform)))

(fn SpawnStoreClosesttoPlayer
  (bind _closesttransfrorm (CallFunction|GetClosestTransformtoPlayer))
  (bind _output_get (LocalVariables|SetSelectedTransform (Transformation|GetActorTransform _closesttransfrorm)))
  (Default|ShowMerchant (Variables|Default|GetShop) _output_get))