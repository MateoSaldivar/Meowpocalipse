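; Barrier manager Blueprint that opens, closes and toggles level barriers held in a Barriers array.
; OpenBarrier ignores its ID, destroying the first barrier and removing it from the array, so later indices shift.
; CloseBarrier and ToggleBarrier set actor collision on the barrier at the given index.
; IsBarrierOpen returns whether collision is enabled, so true means a blocking barrier despite the name.
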(event EventBeginPlay)

(event Collision|EventActorBeginOverlap
  (params (OtherActor :type Actor%20Object%20Reference)))

(event EventTick
  (params (DeltaSeconds :type Float%20%28single-precision%29)))

(fn ConstructionScript)

(fn OpenBarrier
  (params (IdBarrier :type Integer))
  (bind _barriers (Variables|Default|GetBarriers))
  (if (> (Utilities|Array|Length _barriers) 0)
    (Actor|DestroyActor (Utilities|Array|Get(acopy) _barriers))
    (Utilities|Array|RemoveIndex _barriers)))

(fn CloseBarrier
  (params (IdBarrier :type Integer))
  (Collision|SetActorEnableCollision (Utilities|Array|Get(acopy) (Variables|Default|GetBarriers) IdBarrier) true))

(fn ToggleBarrier
  (params (IdBarrier :type Integer))
  (bind _barriers (Variables|Default|GetBarriers))
  (bind _output (Utilities|Array|Get(acopy) _barriers IdBarrier))
  (if (== (Collision|GetActorEnableCollision _output) true)
    (Collision|SetActorEnableCollision _output false)
    (else
      (Collision|SetActorEnableCollision _output true))))

(fn IsBarrierOpen
  (params (IdBarrier :type Integer))
  (return (Collision|GetActorEnableCollision (Utilities|Array|Get(acopy) (Variables|Default|GetBarriers) IdBarrier))))