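; Zone unlocking manager Blueprint, largely a stub for tracking which level zones are unlocked through an UnlockedZones actor array.
; IsZoneUnlocked bounds-checks the index and reports that actor's collision-enabled state as the unlocked flag.
; UnlockZone only performs the bounds check without changing anything, and HandleZoneCompletion, the construction script and the event graph are empty.
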(event EventBeginPlay)

(event Collision|EventActorBeginOverlap
  (params (OtherActor :type Actor%20Object%20Reference)))

(event EventTick
  (params (DeltaSeconds :type Float%20%28single-precision%29)))

(fn ConstructionScript)

(fn UnlockZone
  (params (ZoneIndex :type Integer))
  (if (< ZoneIndex (Utilities|Array|Length (Variables|Default|GetUnlockedZones)))
    _))

(fn IsZoneUnlocked
  (params (ZoneIndex :type Integer))
  (bind _unlockedzones (Variables|Default|GetUnlockedZones))
  (if (< ZoneIndex (Utilities|Array|Length _unlockedzones))
    (return (Collision|GetActorEnableCollision (Utilities|Array|Get(acopy) _unlockedzones ZoneIndex)))))

(fn HandleZoneCompletion)