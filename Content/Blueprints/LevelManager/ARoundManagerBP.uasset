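; Round manager Blueprint that drives zombie spawning between rounds and sets up the level's extraction point.
; StartNewRound increments the round counter and starts the ZombieSpawner, while TransitionToNextRound starts it after a one-shot TimeBetweenRounds timer without incrementing the counter.
; BeginPlay immediately calls CompleteLevel, which hides the ExtractionPoint but enables its collision and tick.
; OpenShop is an empty stub.
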(event Custom|Timer
  (Utilities|Time|SetTimerbyEvent (delegate Custom|Spawn%20Enemys) (Variables|Default|GetTimeBetweenRounds)))

(event Custom|Spawn%20Enemys
  (Default|StartSpawning (Variables|Default|GetZombie%20Spawner%20)))

(event EventBeginPlay
  (CallFunction|CompleteLevel))

(event Collision|EventActorBeginOverlap
  (params (OtherActor :type Actor%20Object%20Reference)))

(event EventTick
  (params (DeltaSeconds :type Float%20%28single-precision%29)))

(fn ConstructionScript)

(fn StartNewRound
  (Variables|Default|SetCurrentRound (+ (Variables|Default|GetCurrentRound) 1))
  (Default|StartSpawning (Variables|Default|GetZombie%20Spawner%20)))

(fn OpenShop)

(fn TransitiontoNextRound
  (CallFunction|Timer))

(fn CompleteLevel
  (bind _extractionpoint (Variables|Default|GetExtractionPoint))
  (Rendering|SetActorHiddenInGame _extractionpoint true)
  (Collision|SetActorEnableCollision _extractionpoint true)
  (Actor|Tick|SetActorTickEnabled _extractionpoint true))