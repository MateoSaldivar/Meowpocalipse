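; ZoneBP is a level-manager zone that tracks its set of barriers and whether the zone is open.
; SetNumBarriers records the starting barrier count, and CheckISopened flags the zone open once the array shrinks below that count or if the count is not positive.
; CheckLastBarrier destroys and removes the sole remaining barrier.
; BeginPlay queries all BarrierIDBP actors, but the result is not stored.
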(event Custom|CheckISopened
  (bind _numbarriers (Variables|Default|GetNumBarriers))
  (if (not (Variables|Default|GetIsOpened))
    (if (> _numbarriers 0)
      (if (< (Utilities|Array|Length (Variables|Default|GetBarriers)) _numbarriers)
        (Variables|Default|SetIsOpened true)
        (else
          (Variables|Default|SetIsOpened false)))
      (else
        (Variables|Default|SetIsOpened true)))))

(event Custom|SetNumBarriers
  (Variables|Default|SetNumBarriers (Utilities|Array|Length (Variables|Default|GetBarriers))))

(event Custom|CheckLastBarrier
  (bind _barriers (Variables|Default|GetBarriers))
  (bind _output (Utilities|Array|Get(acopy) _barriers))
  (if (== (Utilities|Array|Length _barriers) 1)
    (Actor|DestroyActor _output)
    (Utilities|Array|RemoveItem _barriers _output)))

(event EventBeginPlay
  (Actor|GetAllActorsOfClass "/Game/Blueprints/LevelManager/Barriers/BarrierIDBP.BarrierIDBP_C"))

(event Collision|EventActorBeginOverlap
  (params (OtherActor :type Actor%20Object%20Reference)))

(event EventTick
  (params (DeltaSeconds :type Float%20%28single-precision%29)))

(fn ConstructionScript)