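; Zombie agent Blueprint that damages the player on a cooldown while in its attack range and shows directional flipbook animations.
; An overlap volume flags the player, then Tick deals ActorStats attack damage paced by AttackSpeed.
; Incoming damage is forwarded to its own ActorStats component.
; Animation remaps world velocity by the player Prototype's current camera direction, so idle and walk sprites face correctly relative to the view.
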(event OnComponentBeginOverlap(attackRange)
  (params (OverlappedComponent :type Primitive%20Component%20Object%20Reference) (OtherActor :type Actor%20Object%20Reference) (OtherComp :type Primitive%20Component%20Object%20Reference) (OtherBodyIndex :type Integer) (bFromSweep :type Boolean) (SweepResult :type Hit%20Result%20Structure%20%28by%20ref%29))
  (if (== OtherActor (Game|Player|GetPlayerPawn 0))
    (Variables|Default|SetInAttackRange true)))

(event OnComponentEndOverlap(attackRange)
  (params (OverlappedComponent :type Primitive%20Component%20Object%20Reference) (OtherActor :type Actor%20Object%20Reference) (OtherComp :type Primitive%20Component%20Object%20Reference) (OtherBodyIndex :type Integer))
  (if (== OtherActor (Game|Player|GetPlayerPawn 0))
    (Variables|Default|SetInAttackRange false)))

(event Custom|OnTakeAnyDamage_Event
  (params (DamagedActor :type Actor%20Object%20Reference) (Damage :type Float%20%28single-precision%29) (DamageType :type Damage%20Type%20Object%20Reference) (InstigatedBy :type Controller%20Object%20Reference) (DamageCauser :type Actor%20Object%20Reference))
  (Default|StatsTakeDamage (Variables|Default|GetActorStats) Damage))

(event Custom|EventSetAgentState
  (params (State :type State%20Enum :default "NewEnumerator0"))
  (Variables|Default|SetState State))

(event EventBeginPlay
  (EventDispatchers|AssignOnTakeAnyDamage (delegate Custom|OnTakeAnyDamage_Event)))

(event EventTick
  (params (DeltaSeconds :type Float%20%28single-precision%29))
  (CallFunction|Animate)
  (if (Variables|Default|GetInAttackRange)
    (if (<= (Variables|Default|GetattackCoolDown) 0.0)
      (Variables|Default|SetattackCoolDown (Variables|/Game/Agents/Components/ActorStats.ActorStats_C|GetAttackSpeed (Variables|Default|GetActorStats)))
      (CallFunction|DealDamage)
      (else
        (Variables|Default|SetattackCoolDown (- (Variables|Default|GetattackCoolDown) DeltaSeconds))))
    (else
      (Variables|Default|SetattackCoolDown 0.0))))

(fn ConstructionScript)

(fn DealDamage
  (bind _returnvalue (Game|Player|GetPlayerPawn 0))
  (bind _returnvalue_2 (Actor|GetComponentbyClass _returnvalue "/Game/Agents/Components/ActorStats.ActorStats_C"))
  (Default|StatsTakeDamage _returnvalue_2 (Variables|/Game/Agents/Components/ActorStats.ActorStats_C|GetAttack (Variables|Default|GetActorStats)))
  (Development|PrintString (Utilities|String|ToString(Float) (Variables|/Game/Agents/Components/ActorStats.ActorStats_C|GetHP _returnvalue_2))))

(fn Animate
  (bind _animations (LocalVariables|GetAnimations))
  (CallFunction|GetVelwithCamera)
  (if (or (!= (Variables|Default|GetLocalXVel) 0.0) (!= (Variables|Default|GetLocalYVel) 0.0))
    (Variables|Default|SetMoveDirection (select (> (Variables|Default|GetLocalXVel) 0.5) "NewEnumerator3" (select (< (Variables|Default|GetLocalXVel) -0.5) "NewEnumerator2" (select (and (< (Variables|Default|GetLocalYVel) -0.5) (== (Variables|Default|GetLocalXVel) 0.0)) "NewEnumerator1" "NewEnumerator0")))))
  (Sprite|SetFlipbook (Variables|Default|GetCat1_F) (select (> (Math|Vector|VectorLength (Transformation|GetVelocity)) 0.0) (Utilities|Select :Index (Variables|Default|GetMoveDirection) :NewEnumerator0 (.moveup _animations) :NewEnumerator1 (.movedown _animations) :NewEnumerator2 (.moveleft _animations) :NewEnumerator3 (.moveright _animations)) (Utilities|Select :Index (Variables|Default|GetMoveDirection) :NewEnumerator0 (.idleup _animations) :NewEnumerator1 (.idledown _animations) :NewEnumerator2 (.idleleft _animations) :NewEnumerator3 (.idleright _animations)))))

(fn GetVelwithCamera
  (bind _asprototype (Utilities|Casting|CastToPrototype (Game|GetPlayerCharacter 0)))
  (if (== (Variables|/Game/Blueprints/Agents/Prototype.Prototype_C|GetCurrentDirection _asprototype) 1)
    (bind _vel (CallFunction|VelocityDecision false 1.0 -1.0))
    (Variables|Default|SetLocalXVel _vel)
    (bind _vel_2 (CallFunction|VelocityDecision true 1.0 -1.0))
    (Variables|Default|SetLocalYVel _vel_2)
    (elif (== (Variables|/Game/Blueprints/Agents/Prototype.Prototype_C|GetCurrentDirection _asprototype) 2)
      (bind _vel_3 (CallFunction|VelocityDecision true -1.0 1.0))
      (Variables|Default|SetLocalXVel _vel_3)
      (bind _vel_4 (CallFunction|VelocityDecision false 1.0 -1.0))
      (Variables|Default|SetLocalYVel _vel_4)
      (elif (== (Variables|/Game/Blueprints/Agents/Prototype.Prototype_C|GetCurrentDirection _asprototype) 3)
        (bind _vel_5 (CallFunction|VelocityDecision false -1.0 1.0))
        (Variables|Default|SetLocalXVel _vel_5)
        (bind _vel_6 (CallFunction|VelocityDecision true -1.0 1.0))
        (Variables|Default|SetLocalYVel _vel_6)
        (elif (== (Variables|/Game/Blueprints/Agents/Prototype.Prototype_C|GetCurrentDirection _asprototype) 4)
          (bind _vel_7 (CallFunction|VelocityDecision true 1.0 -1.0))
          (Variables|Default|SetLocalXVel _vel_7)
          (bind _vel_8 (CallFunction|VelocityDecision false -1.0 1.0))
          (Variables|Default|SetLocalYVel _vel_8))))))

(fn VelocityDecision
  (params (IsX :type Boolean) (p_true :type Float%20%28double-precision%29) (p_false :type Float%20%28double-precision%29))
  (if IsX
    (return (select (== (Math|Float|Round (.x (Transformation|GetVelocity))) 0) 0.0 (select (> (Math|Float|Round (.x (Transformation|GetVelocity))) 0.5) p_true p_false)))
    (else
      (return (select (== (Math|Float|Round (.y (Transformation|GetVelocity))) 0) 0.0 (select (> (Math|Float|Round (.y (Transformation|GetVelocity))) 0.5) p_true p_false))))))