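; CatBP is a cat agent that follows a Prototype actor once it enters the Sight collision.
; The overlap stores that actor as TargetActor and enables following, which nothing here turns off.
; Every Tick re-issues AIMoveTo toward the target while following is enabled.
; A CheckDistance event that flags closeness within DetectionRad is not called here, and a random-point move near the target is left disconnected.
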(event OnComponentBeginOverlap(Sight)
  (params (OverlappedComponent :type Primitive%20Component%20Object%20Reference) (OtherActor :type Actor%20Object%20Reference) (OtherComp :type Primitive%20Component%20Object%20Reference) (OtherBodyIndex :type Integer) (bFromSweep :type Boolean) (SweepResult :type Hit%20Result%20Structure%20%28by%20ref%29))
  (bind _asprototype (Utilities|Casting|CastToPrototype OtherActor))
  (bind _output_get (Variables|Default|SetTarget%20Actor _asprototype))
  (Variables|Default|SetcanFollowEntity true))

(event Custom|FollowEntity
  (if (Utilities|IsValid (Variables|Default|GetTarget%20Actor))
    (if (Variables|Default|GetcanFollowEntity)
      (AI|AIMoveTo self "0, 0, 0" (stale OnComponentBeginOverlap(Sight) _output_get) 2.0 true))))

(event Custom|CheckDistance
  (Variables|Default|SetCloseToTarget (<= (Transformation|GetDistanceTo self (Variables|Default|GetTarget%20Actor)) (Variables|Default|GetDetection%20Rad))))

(event EventBeginPlay)

(event EventTick
  (params (DeltaSeconds :type Float%20%28single-precision%29))
  (CallFunction|FollowEntity))

(fn ConstructionScript)